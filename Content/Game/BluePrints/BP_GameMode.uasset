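; Game mode that caches the game instance and holds logic to respawn a saved grapple rope (BP_Grappin) in its level.
; SpawnCorde increments Place until GrappinMap has that key, then compares the stored level to the current one.
; On a match, it spawns the grapple at the transform from GrappinPersistant and calls SpawnPersistan, handling only that first key.
; The SpawnCorde call in the event graph is disconnected, so it never runs there.
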(event `self.ReceiveBeginPlay`
  (bind _asbp_game_instance (cast `/Game/Game/BP_GameInstance` (`GameplayStatics.GetGameInstance`)))
  (set `self.As BP Game Instance` _asbp_game_instance))

(fn `UserConstructionScript`)