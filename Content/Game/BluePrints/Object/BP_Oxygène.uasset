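; BP_Oxygène is an interactable oxygen bottle pickup that refills the player's oxygen.
; On interaction it shows the player's bottle sprite, adds its Contenant amount to the Oxygene value in the GameInstance, refreshes the passed widget and destroys itself.
; A box overlap swaps the pickup's sprite to a highlighted version while the player is in range.
; Game instance and player references are cached at BeginPlay.
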(event `self.ReceiveBeginPlay`
  (bind _asbp_game_instance (cast `/Game/Game/BP_GameInstance` (`GameplayStatics.GetGameInstance`)))
  (set `self.As BP Game Instance` _asbp_game_instance)
  (bind _asbp_player (cast `/Game/Game/BluePrints/BP_Player` (`GameplayStatics.GetPlayerPawn` 0)))
  (set `self.As BP Player` _asbp_player))

(event `/Game/Game/Interface/BPI_Interactable.Interactable`
  (params (WidgetRef :type "/Game/Game/Widget/BPW_Main Object Reference"))
  (bind _as_bp_game_instance (`self.As BP Game Instance`))
  (`SceneComponent.SetHiddenInGame` (`/Game/Game/BluePrints/BP_Player.S_Bouteil` (`self.As BP Player`)) false false)
  (set `/Game/Game/BP_GameInstance.Oxygene` (+ (`/Game/Game/BP_GameInstance.Oxygene` _as_bp_game_instance) (`self.Contenant`)) _as_bp_game_instance)
  (`/Game/Game/Widget/BPW_Main.SetOxygene` WidgetRef)
  (`self.K2_DestroyActor`))

(event `self.Box.OnComponentBeginOverlap`
  (params (OverlappedComponent :type "PrimitiveComponent Object Reference") (OtherActor :type "Actor Object Reference") (OtherComp :type "PrimitiveComponent Object Reference") (OtherBodyIndex :type Integer) (bFromSweep :type Boolean) (SweepResult :type "HitResult Structure (by ref)"))
  (cast `/Game/Game/BluePrints/BP_Player` OtherActor)
  (`PaperSpriteComponent.SetSprite` (`self.S_Bouteil`) "/Game/Game/Sprite/Object/Sprite/S_BouteilSelect.S_BouteilSelect"))

(event `self.Box.OnComponentEndOverlap`
  (params (OverlappedComponent :type "PrimitiveComponent Object Reference") (OtherActor :type "Actor Object Reference") (OtherComp :type "PrimitiveComponent Object Reference") (OtherBodyIndex :type Integer))
  (cast `/Game/Game/BluePrints/BP_Player` OtherActor)
  (`PaperSpriteComponent.SetSprite` (`self.S_Bouteil`) "/Game/Game/Sprite/Object/Sprite/S_Bouteil.S_Bouteil"))

(fn `UserConstructionScript`)