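; Grappling hook actor with a physics rope of cube segments and constraints, whose visuals are revealed shortly after spawn.
; PropulseGrappin fires a projectile carrying the hook cube, which freezes in place when its box overlaps something.
; Tick releases an attached, unstuck hook beyond maximum range from the player, and calls StopOldGrappin when rope segments overstretch outside flight.
; Interacting increments the GameInstance grapple count, updates the widget and destroys the hook components.
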(event `self.ReceiveBeginPlay`
  (bind _asbp_player (cast `/Game/Game/BluePrints/BP_Player` (`GameplayStatics.GetPlayerPawn` 0)))
  (set `self.As BP Player` _asbp_player)
  (bind _asbp_game_instance (cast `/Game/Game/BP_GameInstance` (`GameplayStatics.GetGameInstance`)))
  (set `self.As BP Game Instance` _asbp_game_instance)
  (set `self.CordeArray` (`|MakeArray` (`self.Cube1`) (`self.Cube2`) (`self.Cube3`) (`self.Cube4`) (`self.Cube5`) (`self.Cube6`) (`self.Cube7`) (`self.Cube8`) (`self.Cube9`) (`self.Cube10`) (`self.Cube11`) (`self.Cube12`) (`self.Cube13`) (`self.Cube14`) (`self.Cube15`) (`self.Cube16`) (`self.Cube17`) (`self.Cube18`) (`self.Cube19`) (`self.Cube20`) (`self.Cube21`) (`self.Cube22`) (`self.Cube23`)))
  (set `self.PhysicsArray` (`|MakeArray` (`self.PhysicsConstraint1`) (`self.PhysicsConstraint2`) (`self.PhysicsConstraint3`) (`self.PhysicsConstraint4`) (`self.PhysicsConstraint5`) (`self.PhysicsConstraint6`) (`self.PhysicsConstraint7`) (`self.PhysicsConstraint8`) (`self.PhysicsConstraint9`) (`self.PhysicsConstraint10`) (`self.PhysicsConstraint11`) (`self.PhysicsConstraint12`) (`self.PhysicsConstraint13`) (`self.PhysicsConstraint14`) (`self.PhysicsConstraint15`) (`self.PhysicsConstraint16`) (`self.PhysicsConstraint17`) (`self.PhysicsConstraint18`) (`self.PhysicsConstraint19`) (`self.PhysicsConstraint20`) (`self.PhysicsConstraint21`) (`self.PhysicsConstraint22`)))
  (set `self.VisueCordeArray` (`|MakeArray` (`self.S_Corde`) (`self.S_Corde1`) (`self.S_Corde2`) (`self.S_Corde3`) (`self.S_Corde4`) (`self.S_Corde5`) (`self.S_Corde6`) (`self.S_Corde7`) (`self.S_Corde8`) (`self.S_Corde9`) (`self.S_Corde10`) (`self.S_Corde11`) (`self.S_Corde12`) (`self.S_Corde13`) (`self.S_Corde14`) (`self.S_Corde15`) (`self.S_Corde16`) (`self.S_Corde17`) (`self.S_Corde18`) (`self.S_Corde19`) (`self.S_Corde20`) (`self.S_Corde21`) (`self.S_FinCorde`)))
  (`KismetSystemLibrary.Delay` 1.0)
  (for _array_element (`self.VisueCordeArray`)
    (`SceneComponent.SetHiddenInGame` _array_element false false)
    (set `self.Spawn` true)))

(event `CutCorde`
  (params (Target :type "ActorComponent Object Reference"))
  (`/Engine/EditorBlueprintResources/StandardMacros.IsValid` Target
    (:`Is Valid`
      (`ActorComponent.Deactivate` Target)
      (`ActorComponent.K2_DestroyComponent` Target))))

(event `self.ReceiveTick`
  (params (DeltaSeconds :type "Float (single-precision)"))
  (bind _cube (`self.Cube`))
  (if (`self.Spawn`)
    (`|ExecutionSequence`
      (:`then_0`
        (if (`self.IsAttach`)
          (if (`self.IsStuck`)
            _
            (elif (>= (`KismetMathLibrary.Vector_Distance` (`SceneComponent.K2_GetComponentLocation` (`self.Cube`)) (`self.K2_GetActorLocation` (`self.As BP Player`))) 900.0)
              (`/Engine/EditorBlueprintResources/StandardMacros.DoOnce` false
                (:`Completed`
                  (set `self.Stop` true)
                  (`PrimitiveComponent.SetSimulatePhysics` _cube true)
                  (`SceneComponent.K2_DetachFromComponent` _cube "KeepWorld" "KeepWorld" "KeepWorld" true)
                  (`self.K2_DestroyActor` (`self.ProjectilRef`))))))))
      (:`then_1`
        (if (`self.LockLimit`)
          _
          (elif (> (`KismetMathLibrary.Vector_Distance` (`SceneComponent.RelativeLocation` (`self.Cube1`)) (`SceneComponent.RelativeLocation` (`self.Cube2`))) 48.0)
            (`/Game/Game/BluePrints/BP_Player.StopOldGrappin` (`self.As BP Player`))))))))

(event `PropulseGrappin`
  (params (Propulse :type "Float (double-precision)"))
  (set `self.LockLimit` true)
  (bind _returnvalue (`|SpawnActorFromClass` "/Game/Game/BluePrints/Grappin/BP_ProjectilGrappin.BP_ProjectilGrappin_C" (`KismetMathLibrary.MakeTransform` (`SceneComponent.K2_GetComponentLocation` (`self.Cube`)) (`SceneComponent.K2_GetComponentRotation` (`self.Arrow`))) "AlwaysSpawn" "MultiplyWithRoot" null null))
  (bind _output_get (set `self.ProjectilRef` _returnvalue))
  (set `ProjectileMovementComponent.MaxSpeed` Propulse (`/Game/Game/BluePrints/Grappin/BP_ProjectilGrappin.ProjectileMovement` _output_get))
  (`SceneComponent.K2_AttachToComponent` (`self.Cube`) (`/Game/Game/BluePrints/Grappin/BP_ProjectilGrappin.Sphere` _output_get) "None" "SnapToTarget" "KeepWorld" "KeepWorld" true)
  (set `self.CanAttach` true))

(event `self.Box.OnComponentBeginOverlap`
  (params (OverlappedComponent :type "PrimitiveComponent Object Reference") (OtherActor :type "Actor Object Reference") (OtherComp :type "PrimitiveComponent Object Reference") (OtherBodyIndex :type Integer) (bFromSweep :type Boolean) (SweepResult :type "HitResult Structure (by ref)"))
  (bind _cube (`self.Cube`))
  (if (`self.CanAttach`)
    (`PrimitiveComponent.SetSimulatePhysics` _cube false)
    (`SceneComponent.K2_DetachFromComponent` _cube "KeepWorld" "KeepWorld" "KeepWorld" true)
    (set `self.IsStuck` true)
    (set `self.LockLimit` false)
    (`PrimitiveComponent.SetCollisionResponseToChannel` (`self.Cube`) "ECC_GameTraceChannel2" "ECR_Block")
    (if (not (`self.Stop`))
      (`self.K2_DestroyActor` (`self.ProjectilRef`)))))

(event `/Game/Game/Interface/BPI_Interactable.Interactable`
  (params (WidgetRef :type "/Game/Game/Widget/BPW_Main Object Reference"))
  (bind _as_bp_game_instance (`self.As BP Game Instance`))
  (set `/Game/Game/BP_GameInstance.Grappin` (+ (`/Game/Game/BP_GameInstance.Grappin` _as_bp_game_instance) 1) _as_bp_game_instance)
  (`/Game/Game/Widget/BPW_Main.SetGrappin` WidgetRef)
  (`ActorComponent.K2_DestroyComponent` (`self.Cube`))
  (`ActorComponent.K2_DestroyComponent` (`self.Arrow`))
  (`ActorComponent.K2_DestroyComponent` (`self.Box`))
  (`ActorComponent.K2_DestroyComponent` (`self.S_Grappin`)))

(fn `UserConstructionScript`)