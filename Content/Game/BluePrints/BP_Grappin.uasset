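; Grappling hook actor ("Grappin") built from a chain of cube components and launched on BeginPlay by a large impulse on the lead cube, based on the arrow's forward vector.
; A fast looping timer unhides the cubes one after another and makes each block WorldDynamic.
; After a short delay all cubes are constrained to the YZ plane.
; A Box overlap stops physics on the lead cube and reapplies that constraint.
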(event `self.ReceiveBeginPlay`
  (`PrimitiveComponent.AddImpulse` (`self.Cube`) (+ (* (`SceneComponent.GetForwardVector` (`self.Arrow`)) 200000.0) (`self.K2_GetActorLocation`)) "None" false)
  (set `self.Array` (`|MakeArray` (`self.Cube`) (`self.Cube1`) (`self.Cube2`) (`self.Cube3`) (`self.Cube4`) (`self.Cube5`) (`self.Cube6`) (`self.Cube7`) (`self.Cube8`) (`self.Cube9`) (`self.Cube10`) (`self.Cube11`) (`self.Cube12`) (`self.Cube13`) (`self.Cube14`) (`self.Cube15`) (`self.Cube17`) (`self.Cube18`) (`self.Cube19`) (`self.Cube20`) (`self.Cube21`) (`self.Cube22`) (`self.Cube23`) (`self.Cube16`)))
  (set `self.ValueArray` 0)
  (bind _returnvalue (`KismetSystemLibrary.K2_SetTimerDelegate` (delegate `SpawnCollition`) 0.03 true))
  (`KismetSystemLibrary.Delay` 0.5)
  (for _array_element (`self.Array`)
    (`PrimitiveComponent.SetConstraintMode` _array_element "YZPlane")))

(event `SpawnCollition`
  (bind _output (`|GetArrayItem` (`self.Array`) (`self.ValueArray`)))
  (`PrimitiveComponent.SetCollisionResponseToChannel` _output "ECC_WorldDynamic" "ECR_Block")
  (`SceneComponent.SetHiddenInGame` _output false false)
  (if (>= (`self.ValueArray`) (`KismetArrayLibrary.Array_Length` (`self.Array`)))
    (`KismetSystemLibrary.K2_PauseTimerHandle` (stale `self.ReceiveBeginPlay` _returnvalue))
    (else
      (set `self.ValueArray` (+ (`self.ValueArray`) 1)))))

(event `self.Box.OnComponentBeginOverlap`
  (params (OverlappedComponent :type "PrimitiveComponent Object Reference") (OtherActor :type "Actor Object Reference") (OtherComp :type "PrimitiveComponent Object Reference") (OtherBodyIndex :type Integer) (bFromSweep :type Boolean) (SweepResult :type "HitResult Structure (by ref)"))
  (`PrimitiveComponent.SetSimulatePhysics` (`self.Cube`) false)
  (for _array_element (`self.Array`)
    (`PrimitiveComponent.SetConstraintMode` _array_element "YZPlane")))

(fn `UserConstructionScript`)