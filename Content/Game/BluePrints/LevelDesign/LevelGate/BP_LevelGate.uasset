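; BP_LevelGate is a level transition door that sends the player to another level and places them at the matching gate on arrival.
; When the player overlaps its Box, it saves its PorteRef to PorteArriver on BP_GameInstance, then opens the referenced Level.
; On BeginPlay, a gate whose PorteRef equals that saved value moves the player to its Arrow's location, using the Game Instance to carry state across loads.
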(event `self.ReceiveBeginPlay`
  (bind _asbp_player (cast `/Game/Game/BluePrints/BP_Player` (`GameplayStatics.GetPlayerPawn` 0)))
  (set `self.As BP Player` _asbp_player)
  (bind _asbp_game_instance (cast `/Game/Game/BP_GameInstance` (`GameplayStatics.GetGameInstance`)))
  (set `self.As BP Game Instance` _asbp_game_instance)
  (if (== (`/Game/Game/BP_GameInstance.PorteArriver` (`self.As BP Game Instance`)) (`self.PorteRef`))
    (`self.K2_SetActorLocation` (`self.As BP Player`) (`SceneComponent.K2_GetComponentLocation` (`self.Arrow`)) false false)))

(event `self.Box.OnComponentBeginOverlap`
  (params (OverlappedComponent :type "PrimitiveComponent Object Reference") (OtherActor :type "Actor Object Reference") (OtherComp :type "PrimitiveComponent Object Reference") (OtherBodyIndex :type Integer) (bFromSweep :type Boolean) (SweepResult :type "HitResult Structure (by ref)"))
  (cast `/Game/Game/BluePrints/BP_Player` OtherActor)
  (set `/Game/Game/BP_GameInstance.PorteArriver` (`self.PorteRef`) (`self.As BP Game Instance`))
  (`GameplayStatics.OpenLevelBySoftObjectPtr` (`self.Level`)))

(fn `UserConstructionScript`)