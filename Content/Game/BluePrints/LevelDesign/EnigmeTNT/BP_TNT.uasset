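; BP_TNT is an explosive prop, apparently for a TNT level puzzle, that blows up when its Detonate event is called.
; Detonate waits a random fraction of a second to a few seconds, then plays a 2D explosion sound.
; A multi sphere trace at its location sends DestroyMessage to every hit actor implementing BPI_Destructible, then the TNT destroys itself.
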(event `self.ReceiveBeginPlay`)

(event `/Game/Game/Interface/BPI_Explosif.Detonate`
  (bind _returnvalue (`self.K2_GetActorLocation`))
  (`KismetSystemLibrary.Delay` (`KismetMathLibrary.RandomFloatInRange` 0.5 5.0))
  (`GameplayStatics.PlaySound2D` "/Game/StarterContent/Audio/Explosion01.Explosion01" 1.0 1.0 0.0 null null)
  (bind _outhits (`KismetSystemLibrary.SphereTraceMulti` _returnvalue _returnvalue 500.0 "TraceTypeQuery5"))
  (for _array_element _outhits
    (bind (_bblockinghit _binitialoverlap _time _distance _location _impactpoint _normal _impactnormal _physmat _hitactor) (`GameplayStatics.BreakHitResult` _array_element))
    (if (`KismetSystemLibrary.DoesImplementInterface` _hitactor "/Game/Game/Interface/BPI_Destructible.BPI_Destructible_C")
      (message `/Game/Game/Interface/BPI_Destructible.Destroy` _hitactor)))
  (`self.K2_DestroyActor`))

(fn `UserConstructionScript`)