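; Interactable detonator for the TNT puzzle, a sprite actor that highlights while the player overlaps its box.
; On interaction, it counts primed entries in the GameInstance's AmorceState array, treating the first three indices as good and the rest as bad.
; Three bad primers play an explosion and quit the game; otherwise three good ones message every BP_TNT to detonate.
; Any other result resets the sprite and DoOnce for another try.
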(event `self.ReceiveBeginPlay`
  (bind _asbp_game_instance (cast `/Game/Game/BP_GameInstance` (`GameplayStatics.GetGameInstance`)))
  (set `self.As BP Game Instance` _asbp_game_instance))

(event `/Game/Game/Interface/BPI_Interactable.Interactable`
  (params (WidgetRef :type "/Game/Game/Widget/BPW_PlayerScreen Object Reference"))
  (`/Engine/EditorBlueprintResources/StandardMacros.DoOnce` false :!label _label
    (:`Completed`
      (set `self.BadAmorce` 0)
      (set `self.GoodAmorce` 0)
      (set `self.Count` 0)
      (for (_array_element _array_index) (`/Game/Game/BP_GameInstance.AmorceState` (`self.As BP Game Instance`))
        (if (>= _array_index 3)
          (if (== _array_element true)
            (set `self.BadAmorce` (+ (`self.BadAmorce`) 1)))
          (elif (== _array_element true)
            (bind _output_get (set `self.GoodAmorce` (+ (`self.GoodAmorce`) 1)))
            (`KismetSystemLibrary.PrintString` (`KismetStringLibrary.Conv_IntToString` _output_get)))))
      (set `self.Activate` true)
      (`PaperSpriteComponent.SetSprite` (`self.PaperSprite`) "/Game/Game/Sprite/Object/Sprite/S_DetonateurActive.S_DetonateurActive")
      (if (== (`self.BadAmorce`) 3)
        (`GameplayStatics.PlaySound2D` "/Game/StarterContent/Audio/Explosion01.Explosion01" 2.0 1.0 0.0 null null)
        (`KismetSystemLibrary.Delay` 2.0)
        (`KismetSystemLibrary.QuitGame` null "Quit")
        (elif (== (`self.GoodAmorce`) 3)
          (bind _outactors (`GameplayStatics.GetAllActorsOfClass` "/Game/Game/BluePrints/LevelDesign/EnigmeTNT/BP_TNT.BP_TNT_C"))
          (for _array_element_2 _outactors
            (message `/Game/Game/Interface/BPI_Explosif.Detonate` _array_element_2))
          (else
            (`KismetSystemLibrary.Delay` 0.2)
            (`PaperSpriteComponent.SetSprite` (`self.PaperSprite`) "/Game/Game/Sprite/Object/Sprite/S_Detonateur.S_Detonateur")
            (set `self.Activate` false)
            (goto _label :!via `Reset`)))))))

(event `self.Box.OnComponentBeginOverlap`
  (params (OverlappedComponent :type "PrimitiveComponent Object Reference") (OtherActor :type "Actor Object Reference") (OtherComp :type "PrimitiveComponent Object Reference") (OtherBodyIndex :type Integer) (bFromSweep :type Boolean) (SweepResult :type "HitResult Structure (by ref)"))
  (cast `/Game/Game/BluePrints/BP_Player` OtherActor)
  (if (not (`self.Activate`))
    (`PaperSpriteComponent.SetSprite` (`self.PaperSprite`) "/Game/Game/Sprite/Object/Sprite/S_DetonateurInteract.S_DetonateurInteract")))

(event `self.Box.OnComponentEndOverlap`
  (params (OverlappedComponent :type "PrimitiveComponent Object Reference") (OtherActor :type "Actor Object Reference") (OtherComp :type "PrimitiveComponent Object Reference") (OtherBodyIndex :type Integer))
  (cast `/Game/Game/BluePrints/BP_Player` OtherActor)
  (if (not (`self.Activate`))
    (`PaperSpriteComponent.SetSprite` (`self.PaperSprite`) "/Game/Game/Sprite/Object/Sprite/S_Detonateur.S_Detonateur")))

(fn `UserConstructionScript`)