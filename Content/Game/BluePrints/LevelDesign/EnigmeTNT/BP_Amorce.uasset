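; BP_Amorce is a primer for the TNT puzzle that the player activates through its Interactable event.
; Its box overlap with BP_Player toggles the sprite between inactive and interact-highlight until it is active.
; Interacting switches to the active sprite and records the state at its Index in BP_GameInstance's AmorceState array, which BeginPlay reads to restore already-activated primers.
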(event `self.ReceiveBeginPlay`
  (bind _asbp_game_instance (cast `/Game/Game/BP_GameInstance` (`GameplayStatics.GetGameInstance`)))
  (bind _output_get (set `self.As BP Game Instance` _asbp_game_instance))
  (if (`|GetArrayItem` (`/Game/Game/BP_GameInstance.AmorceState` _output_get) (`self.Index`))
    (`PaperSpriteComponent.SetSprite` (`self.PaperSprite`) "/Game/Game/Sprite/Object/Sprite/S_AmorceActive.S_AmorceActive")
    (set `self.IsActive` true)))

(event `/Game/Game/Interface/BPI_Interactable.Interactable`
  (params (WidgetRef :type "/Game/Game/Widget/BPW_PlayerScreen Object Reference"))
  (`PaperSpriteComponent.SetSprite` (`self.PaperSprite`) "/Game/Game/Sprite/Object/Sprite/S_AmorceActive.S_AmorceActive")
  (`KismetArrayLibrary.Array_Set` (`/Game/Game/BP_GameInstance.AmorceState` (`self.As BP Game Instance`)) (`self.Index`) true)
  (set `self.IsActive` true))

(event `self.Box.OnComponentBeginOverlap`
  (params (OverlappedComponent :type "PrimitiveComponent Object Reference") (OtherActor :type "Actor Object Reference") (OtherComp :type "PrimitiveComponent Object Reference") (OtherBodyIndex :type Integer) (bFromSweep :type Boolean) (SweepResult :type "HitResult Structure (by ref)"))
  (cast `/Game/Game/BluePrints/BP_Player` OtherActor)
  (if (not (`self.IsActive`))
    (`PaperSpriteComponent.SetSprite` (`self.PaperSprite`) "/Game/Game/Sprite/Object/Sprite/S_AmorceInteract.S_AmorceInteract")))

(event `self.Box.OnComponentEndOverlap`
  (params (OverlappedComponent :type "PrimitiveComponent Object Reference") (OtherActor :type "Actor Object Reference") (OtherComp :type "PrimitiveComponent Object Reference") (OtherBodyIndex :type Integer))
  (cast `/Game/Game/BluePrints/BP_Player` OtherActor)
  (if (not (`self.IsActive`))
    (`PaperSpriteComponent.SetSprite` (`self.PaperSprite`) "/Game/Game/Sprite/Object/Sprite/S_AmorceInactive.S_AmorceInactive")))

(fn `UserConstructionScript`)