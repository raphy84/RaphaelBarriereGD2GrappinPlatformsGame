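; BP_Pick is a level-design actor that severs a BP_Grappin grappling rope on contact with its Box trigger.
; On overlap, it searches the grapple's CordeArray for the touched component, then clears and destroys the physics constraint at the same index in PhysicsArray.
; With no match, the index stays on the last element looped over, so that constraint is destroyed instead.
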(event `self.Box.OnComponentBeginOverlap`
  (params (OverlappedComponent :type "PrimitiveComponent Object Reference") (OtherActor :type "Actor Object Reference") (OtherComp :type "PrimitiveComponent Object Reference") (OtherBodyIndex :type Integer) (bFromSweep :type Boolean) (SweepResult :type "HitResult Structure (by ref)"))
  (bind _asbp_grappin (cast `/Game/Game/BluePrints/Grappin/BP_Grappin` OtherActor))
  (for (_array_element _array_index) (`/Game/Game/BluePrints/Grappin/BP_Grappin.CordeArray` _asbp_grappin)
    (set `self.DestroyArray` _array_index)
    (if (== _array_element OtherComp)
      (break)))
  (bind _output (`|GetArrayItem` (`/Game/Game/BluePrints/Grappin/BP_Grappin.PhysicsArray` _asbp_grappin) (`self.DestroyArray`)))
  (`PhysicsConstraintComponent.SetConstrainedComponents` _output null "None" null "None")
  (`ActorComponent.K2_DestroyComponent` _output))

(fn `UserConstructionScript`)