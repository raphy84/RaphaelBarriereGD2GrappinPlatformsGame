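; Player character for a grappling-hook game with movement aimed on a constant-X plane, a detached camera and gold pickups.
; Mouse rays intersect that plane to rotate an aim arrow, along which Shoot spawns limited BP_Grappin hooks; Reset destroys and refills them.
; Capsule overlaps attach the player to hooks while right mouse is held (R detaches, F applies impulse) and collect loot, updating GameInstance counters and the HUD.
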(event `self.ReceiveBeginPlay`
  (bind _returnvalue (`|CreateWidget` "/Game/Game/Widget/BPW_Main.BPW_Main_C"))
  (bind _output_get (set `self.MainWidgetRef` _returnvalue))
  (`UserWidget.AddToPlayerScreen` _output_get 0)
  (bind _asbp_game_instance (cast `/Game/Game/BP_GameInstance` (`GameplayStatics.GetGameInstance`)))
  (set `self.As BP Game Instance` _asbp_game_instance)
  (bind _asplayer_controller (cast `PlayerController` (`self.GetController`)))
  (bind _returnvalue_2 (pcsubsystem `EnhancedInputLocalPlayerSubsystem` _asplayer_controller))
  (`/Engine/EditorBlueprintResources/StandardMacros.IsValid` _returnvalue_2
    (:`Is Valid`
      (`EnhancedInputSubsystemInterface.AddMappingContext` _returnvalue_2 "/Game/Game/Input/IMC_Default.IMC_Default" 0 (struct))
      (`SceneComponent.K2_DetachFromComponent` (`self.Camera`) "KeepWorld" "KeepWorld" "KeepWorld" true))))

(event `self.ReceiveTick`
  (params (DeltaSeconds :type "Float (single-precision)"))
  (bind (_worldlocation _worlddirection) (`PlayerController.DeprojectMousePositionToWorld` (`GameplayStatics.GetPlayerController` 0)))
  (`PhysicsHandleComponent.SetTargetLocation` (`self.PhysicsHandle`) (`self.K2_GetActorLocation`))
  (bind _aimgrappin (`self.AimLocation` _worldlocation (+ _worldlocation (* _worlddirection 1000000.0))))
  (`KismetSystemLibrary.DrawDebugSphere` _aimgrappin 20.0 12 (struct :`G` 1.0 :`B` 0.157874 :`A` 1.0))
  (bind (_yaw _pitch) (`KismetMathLibrary.GetYawPitchFromVector` (`KismetMathLibrary.Normal` (- (`SceneComponent.K2_GetComponentLocation` (`self.Arrow1`)) _aimgrappin))))
  (`SceneComponent.K2_SetWorldRotation` (`self.Arrow1`) (`KismetMathLibrary.MakeRotator` 0.0 _pitch _yaw) false false))

(event `EnhancedInput|/Game/Game/Actions/IA_Move`
  (params (ActionValue :type "Float (double-precision)") (ElapsedSeconds :type "Float (double-precision)") (TriggeredSeconds :type "Float (double-precision)") (InputAction :type "InputAction Object Reference" :default "/Game/Game/Actions/IA_Move.IA_Move"))
  (bind _charactermovement (`self.CharacterMovement`))
  (bind (_velocity_x _velocity_y _velocity_z) (`KismetMathLibrary.BreakVector` (`MovementComponent.Velocity` _charactermovement)))
  (:`Triggered`
    (`self.AddMovementInput` (`self.GetActorForwardVector`) ActionValue true))
  (:`Completed`
    (set `MovementComponent.Velocity` (`KismetMathLibrary.MakeVector` 0.0 (/ _velocity_y 5.0) _velocity_z) _charactermovement)))

(event `EnhancedInput|/Game/Game/Actions/IA_Shoot`
  (params (ActionValue :type Boolean) (ElapsedSeconds :type "Float (double-precision)") (TriggeredSeconds :type "Float (double-precision)") (InputAction :type "InputAction Object Reference" :default "/Game/Game/Actions/IA_Shoot.IA_Shoot"))
  (bind _as_bp_game_instance (`self.As BP Game Instance`))
  (:`Started`
    (if (not (<= (`/Game/Game/BP_GameInstance.Grappin` (`self.As BP Game Instance`)) 0))
      (`|SpawnActorFromClass` "/Game/Game/BluePrints/BP_Grappin.BP_Grappin_C" (`KismetMathLibrary.MakeTransform` (+ (`self.K2_GetActorLocation`) (0.0 0.0 50.0)) (`KismetMathLibrary.MakeRotFromYX` (`KismetMathLibrary.NegateVector` (`KismetMathLibrary.GetForwardVector` (`SceneComponent.K2_GetComponentRotation` (`self.Arrow1`)))) (1.0 0.0 0.0))) "AlwaysSpawn" "MultiplyWithRoot" null null)
      (set `/Game/Game/BP_GameInstance.Grappin` (- (`/Game/Game/BP_GameInstance.Grappin` _as_bp_game_instance) 1) _as_bp_game_instance)
      (`/Game/Game/Widget/BPW_Main.SetGrappin` (`self.MainWidgetRef`)))))

(event `EnhancedInput|/Game/Game/Actions/IA_Jump`
  (params (ActionValue :type Boolean) (ElapsedSeconds :type "Float (double-precision)") (TriggeredSeconds :type "Float (double-precision)") (InputAction :type "InputAction Object Reference" :default "/Game/Game/Actions/IA_Jump.IA_Jump"))
  (:`Triggered`
    (`KismetSystemLibrary.DelayUntilNextTick`)
    (if (`NavMovementComponent.IsFalling` (`self.CharacterMovement`))
      (if (`self.AttachGrappin`)
        (`self.LaunchCharacter` (0.0 0.0 50.0)))
      (else
        (`self.LaunchCharacter` (0.0 0.0 500.0))))))

(event `EnhancedInput|/Game/Game/Actions/IA_Reset`
  (params (ActionValue :type Boolean) (ElapsedSeconds :type "Float (double-precision)") (TriggeredSeconds :type "Float (double-precision)") (InputAction :type "InputAction Object Reference" :default "/Game/Game/Actions/IA_Reset.IA_Reset"))
  (bind _as_bp_game_instance (`self.As BP Game Instance`))
  (:`Triggered`
    (bind _outactors (`GameplayStatics.GetAllActorsOfClass` "/Game/Game/BluePrints/BP_Grappin.BP_Grappin_C"))
    (for _array_element _outactors
      (`self.K2_DestroyActor` _array_element)
      (set `/Game/Game/BP_GameInstance.Grappin` (`/Game/Game/BP_GameInstance.GrappinMax` _as_bp_game_instance) _as_bp_game_instance)
      (`/Game/Game/Widget/BPW_Main.SetGrappin` (`self.MainWidgetRef`)))))

(event `self.CapsuleComponent.OnComponentBeginOverlap`
  (params (OverlappedComponent :type "PrimitiveComponent Object Reference") (OtherActor :type "Actor Object Reference") (OtherComp :type "PrimitiveComponent Object Reference") (OtherBodyIndex :type Integer) (bFromSweep :type Boolean) (SweepResult :type "HitResult Structure (by ref)"))
  (bind _as_bp_game_instance (`self.As BP Game Instance`))
  (bind _as_bp_game_instance_2 (`self.As BP Game Instance`))
  (cast `/Game/Game/BluePrints/BP_Grappin` OtherActor
    (:`then`
      (set `self.AttachGrappin` true)
      (set `self.Other Comp` OtherComp)
      (if (`self.Can attach`)
        (`/Engine/EditorBlueprintResources/StandardMacros.DoOnce` false :!label _label
          (:`Completed`
            (`self.K2_AttachToComponent` (`self.Other Comp`) "None" "SnapToTarget" "KeepWorld" "KeepWorld")
            (`ActorComponent.Deactivate` (`self.PhysicsHandle`))
            (set `CharacterMovementComponent.Mass` 0.0 (`self.CharacterMovement`))))))
    (:`CastFailed`
      (if (`KismetSystemLibrary.DoesImplementInterface` OtherActor "/Game/Game/Interface/BPI_Interactable.BPI_Interactable_C")
        (bind _asbp_gold (cast `/Game/Game/BluePrints/BP_Gold` OtherActor)
          (:`then`
            (`/Game/Game/BluePrints/BP_Gold.Interactable` _asbp_gold)
            (set `/Game/Game/BP_GameInstance.Gold` (+ (`/Game/Game/BP_GameInstance.Gold` _as_bp_game_instance) 1) _as_bp_game_instance)
            (`/Game/Game/Widget/BPW_Main.SetGold` (`self.MainWidgetRef`)))
          (:`CastFailed`
            (bind _asbp_grappin_loot (cast `/Game/Game/BluePrints/BP_GrappinLoot` OtherActor))
            (`/Game/Game/BluePrints/BP_GrappinLoot.Interactable` _asbp_grappin_loot)
            (set `/Game/Game/BP_GameInstance.Grappin` (+ (`/Game/Game/BP_GameInstance.Grappin` _as_bp_game_instance_2) 1) _as_bp_game_instance_2)
            (set `/Game/Game/BP_GameInstance.GrappinMax` (+ (`/Game/Game/BP_GameInstance.GrappinMax` _as_bp_game_instance_2) 1) _as_bp_game_instance_2)
            (`/Game/Game/Widget/BPW_Main.SetGrappin` (`self.MainWidgetRef`))))))))

(event `self.CapsuleComponent.OnComponentEndOverlap`
  (params (OverlappedComponent :type "PrimitiveComponent Object Reference") (OtherActor :type "Actor Object Reference") (OtherComp :type "PrimitiveComponent Object Reference") (OtherBodyIndex :type Integer))
  (cast `/Game/Game/BluePrints/BP_Grappin` OtherActor)
  (set `self.AttachGrappin` false))

(event `Key|RightMouseButton`
  (params (Key :type "Key Structure"))
  (:`Pressed`
    (set `self.Can attach` true))
  (:`Released`
    (set `self.Can attach` false)))

(event `Key|R`
  (params (Key :type "Key Structure"))
  (:`Pressed`
    (`self.K2_DetachFromActor` "KeepWorld" "KeepWorld" "KeepWorld")
    (`self.K2_SetActorRotation` (struct))
    (goto _label :!via `Reset`)))

(event `Key|F`
  (params (Key :type "Key Structure"))
  (:`Pressed`
    (`PrimitiveComponent.AddImpulse` (`self.Other Comp`) (0.0 50000.0 0.0) "None" false)))

(fn `AimLocation`
  (params (InputLocation :type "Vector Structure") (InputDirection :type "Vector Structure"))
  (returns (AimGrappin :type "Vector Structure"))
  (bind _x (.x InputLocation))
  (bind _y (.y InputLocation))
  (bind _z (.z InputLocation))
  (bind _x_2 (.x InputDirection))
  (bind _returnvalue_x (`KismetMathLibrary.BreakVector` (`self.K2_GetActorLocation`)))
  (return (`KismetMathLibrary.MakeVector` _returnvalue_x (+ (/ (* (- _returnvalue_x _x) (- (.y InputDirection) _y)) (- _x_2 _x)) _y) (+ _z (/ (* (- _returnvalue_x _x) (- (.z InputDirection) _z)) (- _x_2 _x))))))

(fn `UserConstructionScript`)